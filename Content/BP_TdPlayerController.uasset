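; Player controller, apparently for a TD game mode, that owns the main HUD and pause menu.
; On BeginPlay it creates the HUD widget and adds it to the viewport.
; The Enhanced Input pause action either opens a pause menu, pausing and showing the cursor, or closes a valid stored menu and restores game-only input.
; The open branch clears its stored menu reference immediately, so the close branch is not reached on later presses.
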(event `self.ReceiveBeginPlay`
  ; Main HUD Logic
  (bind _returnvalue (`|CreateWidget` "/Game/UI/WBP_MainHUD.WBP_MainHUD_C"))
  (`UserWidget.AddToViewport` _returnvalue 0))

(event `EnhancedInput|/Game/Input/IA_Pause`
  (params (ActionValue :type Boolean) (ElapsedSeconds :type "Float (double-precision)") (TriggeredSeconds :type "Float (double-precision)") (InputAction :type "InputAction Object Reference" :default "/Game/Input/IA_Pause.IA_Pause"))
  ; Pause Triggered
  (:`Started`
    (bind _activepausemenu (`self.ActivePauseMenu`)
      (:`then`
        (`Widget.RemoveFromParent` _activepausemenu)
        (`GameplayStatics.SetGamePaused` false)
        (`WidgetBlueprintLibrary.SetInputMode_GameOnly` (`GameplayStatics.GetPlayerController` 0))
        (set `self.bShowMouseCursor` false))
      (:`else`
        (bind _returnvalue (`|CreateWidget` "/Game/UI/WBP_PauseMenu.WBP_PauseMenu_C"))
        (set `self.ActivePauseMenu` _returnvalue)
        (`UserWidget.AddToViewport` _returnvalue 0)
        (`GameplayStatics.SetGamePaused` true)
        (set `self.bShowMouseCursor` true)
        (set `self.ActivePauseMenu` null)))))

(fn `UserConstructionScript`)