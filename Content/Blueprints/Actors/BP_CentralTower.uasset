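; BP_CentralTower is the clickable central tower whose death ends the game.
; BeginPlay creates a dynamic body material, links a green health bar widget to Health and binds death to a handler that shows the game-over screen and pauses.
; Clicking calls Upgrade, defined outside these graphs.
; A separate, locally uncalled event sets the material's upgrade level and has Niagara upgrade effects behind a switch fixed at 0, so neither spawns.
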(event `self.ReceiveBeginPlay`
  ; health and Gameover screen
  (bind _returnvalue (`PrimitiveComponent.CreateDynamicMaterialInstance` (`self.Mesh`) 0 "/Game/Materials/M_Defender_Upgradeable.M_Defender_Upgradeable" "None"))
  (set `self.MID_Body` _returnvalue)
  (bind _aswbp_health_bar (cast `/Game/UI/WBP_HealthBar` (`WidgetComponent.GetUserWidgetObject` (`self.HealthWidget`))))
  (`/Game/UI/WBP_HealthBar.SetBarColor` _aswbp_health_bar (struct :`G` 1.0 :`A` 1.0))
  (set `/Game/UI/WBP_HealthBar.HealthReference` (`self.Health`) _aswbp_health_bar)
  (add `HealthComponent.OnDeath` (`self.Health`) (delegate `HandleGameOver`)))

(event `HandleGameOver`
  (bind _returnvalue (`GameplayStatics.GetPlayerController` 0))
  ; health and Gameover screen
  (bind _returnvalue_2 (`|CreateWidget` "/Game/UI/WBP_GameOver.WBP_GameOver_C"))
  (`UserWidget.AddToViewport` _returnvalue_2 0)
  (`WidgetBlueprintLibrary.SetInputMode_UIOnlyEx` _returnvalue null)
  (set `PlayerController.bShowMouseCursor` true _returnvalue)
  (`GameplayStatics.SetGamePaused` true))

(event `CustomEvent`
  (`MaterialInstanceDynamic.SetScalarParameterValue` (`self.MID_Body`) "UpgradeLevel" (`KismetMathLibrary.Conv_IntToDouble` (`self.CurrentLevel`)))
  (switch `int` 0
    (:`1`
      (`NiagaraFunctionLibrary.SpawnSystemAttached` "/Game/Blueprints/VFX/NS_Upgrade_L1.NS_Upgrade_L1" (`self.Mesh`) "None" (0.0 0.0 0.0) (struct) "SnapToTarget" true))
    (:`2`
      (`NiagaraFunctionLibrary.SpawnSystemAttached` "/Game/Blueprints/VFX/NS_Upgrade_L2.NS_Upgrade_L2" (`self.Mesh`) "None" (0.0 0.0 0.0) (struct) "SnapToTarget" true))))

(event `self.ReceiveActorOnClicked`
  (params (ButtonPressed :type "Key Structure"))
  (`self.Upgrade`))

(fn `UserConstructionScript`)